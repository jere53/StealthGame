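; AI controller for stealth guards that runs BT_Guard and feeds sight perception into its blackboard.
; Perception updates are routed by the sense class's display name, with only sight shown handled.
; Any sight update sets IsInvestigating to whether sensing succeeded; seeing player 0 also sets the target actor and changes guard walk speed.
; Losing sight stores the stimulus location and clears the target actor, without restoring speed here.
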(event OnTargetPerceptionUpdated(AIPerception)
  (params (Actor :type Actor%20Object%20Reference) (Stimulus :type AI%20Stimulus%20Structure))
  (bind _returnvalue (Class|AIPerceptionSystem|GetSenseClassforStimulus Stimulus))
  (CallFunction|HandleSense (Utilities|GetClassDisplayName _returnvalue) Stimulus Actor))

(event EventBeginPlay
  (AI|RunBehaviorTree "/Game/StealthGame/AI/BT_Guard.BT_Guard"))

(event EventTick
  (params (DeltaSeconds :type Float%20%28single-precision%29)))

(fn ConstructionScript)

(fn HandleSense
  (params (Selection :type String) (Stimulus :type AI%20Stimulus%20Structure) (SensedActor :type Actor%20Object%20Reference))
  (bind _blackboard (Variables|Default|GetBlackboard))
  (bind _blackboard_2 (Variables|Default|GetBlackboard))
  (switch string Selection
    (:AiSense_Sight
      (AI|Components|Blackboard|SetValueasBool _blackboard (Utilities|Name|MakeLiteralName "IsInvestigating") (.bsuccessfullysensed Stimulus))
      (if (.bsuccessfullysensed Stimulus)
        (if (== SensedActor (Game|GetPlayerCharacter 0))
          (AI|Components|Blackboard|SetValueasObject _blackboard_2 (Utilities|Name|MakeLiteralName "TargetLocationActor") SensedActor)
          (bind _ascharacter (Utilities|Casting|CastToCharacter (Pawn|GetControlledPawn)))
          (Variables|/Script/Engine.CharacterMovementComponent|SetMaxWalkSpeed (Variables|/Script/Engine.Character|GetCharacterMovement _ascharacter) 4e+02))
        (else
          (AI|Components|Blackboard|SetValueasVector _blackboard (Utilities|Name|MakeLiteralName "TargetLocationVector") (.stimuluslocation Stimulus))
          (AI|Components|Blackboard|SetValueasObject _blackboard_2 (Utilities|Name|MakeLiteralName "TargetLocationActor") 0))))))