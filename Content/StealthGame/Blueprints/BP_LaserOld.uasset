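; Laser actor that renders a Niagara beam along its forward vector, stopping at the first blocking surface.
; Each Tick it line-traces on Visibility up to Distance, sets the beam's "Laser End" parameter to the hit or maximum range, and shows the impact effect only on a hit.
; The Construction Script previews a green, untraced beam from the Sphere component's forward vector; BeginPlay switches it to red.
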(event EventBeginPlay
  (Effects|Components|ParticleSystem|SetColorParameter (Variables|Default|GetNiagaraLaser) "Color" "(R=1.000000,G=0.000000,B=0.009947,A=1.000000)")
  (Effects|Components|ParticleSystem|SetColorParameter (Variables|Default|GetNiagaraLaserImpact) "Color" "(R=1.000000,G=0.000000,B=0.009947,A=1.000000)"))

(event Collision|EventActorBeginOverlap
  (params (OtherActor :type Actor%20Object%20Reference)))

(event EventTick
  (params (DeltaSeconds :type Float%20%28single-precision%29))
  (bind _returnvalue (Transformation|GetActorLocation))
  (bind _returnvalue_2 (Transformation|GetActorForwardVector))
  (bind _distance (Variables|Default|GetDistance))
  (bind _niagaralaserimpact (Variables|Default|GetNiagaraLaserImpact))
  (bind _returnvalue_3 (* _returnvalue_2 _distance))
  (bind _returnvalue_4 (+ _returnvalue _returnvalue_3))
  (bind _outhit (Collision|LineTraceByChannel _returnvalue _returnvalue_4 "TraceTypeQuery1" false 0 "None"))
  (Effects|Components|ParticleSystem|SetVectorParameter (Variables|Default|GetNiagaraLaser) "Laser End" (select (.bBlockingHit (Collision|BreakHitResult _outhit)) (.Location (Collision|BreakHitResult _outhit)) _returnvalue_4))
  (Rendering|SetVisibility _niagaralaserimpact (.bBlockingHit (Collision|BreakHitResult _outhit)) false)
  (Transformation|SetWorldLocation _niagaralaserimpact (.Location (Collision|BreakHitResult _outhit)) false false))

(fn ConstructionScript
  (bind _sphere (Variables|Default|GetSphere))
  (Effects|Components|ParticleSystem|SetColorParameter (Variables|Default|GetNiagaraLaser) "Color" "(R=0.000000,G=1.000000,B=0.480082,A=1.000000)")
  (Effects|Components|ParticleSystem|SetColorParameter (Variables|Default|GetNiagaraLaserImpact) "Color" "(R=1.000000,G=0.000000,B=0.009947,A=1.000000)")
  (Effects|Components|ParticleSystem|SetVectorParameter (Variables|Default|GetNiagaraLaser) "Laser End" (+ (Transformation|GetWorldLocation _sphere) (* (Math|Vector|GetForwardVector _sphere) (Variables|Default|GetDistance)))))